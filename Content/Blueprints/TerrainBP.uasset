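; Terrain actor that builds the playable map at BeginPlay from the grid data in Cell.
; It adds a floor instance, then stacks randomly rotated rock instances on every tile marked 1, using instancing rather than separate actors.
; It then spawns FeatherPickup actors at Cell's feather locations, converting grid indices to offset world positions.
; The construction script is empty, with a similar floor-and-rock build left unconnected.
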(event EventBeginPlay
  (bind _cell (Variables|Default|GetCell))
  (bind _gridsize (Variables|/Script/GameJam.CellularTerrain|GetGridSize _cell))
  (Components|InstancedStaticMesh|AddInstance (Variables|Default|GetFloor) (Math|Conversions|ToTransform(Vector) (Math|Vector|MakeVector 25.0 25.0 0.0)))
  (for _index (range 0 _gridsize)
    (for _index_2 (range 0 _gridsize)
      (bind _returnvalue (Class|CellularTerrain|GetIndex _cell _index _index_2))
      (if (== (Utilities|Array|Get(acopy) (Variables|/Script/GameJam.CellularTerrain|GetTileGrid _cell) _returnvalue) 1)
        (for _index_3 (range 0 2)
          (Components|InstancedStaticMesh|AddInstance (Variables|Default|GetRock%204) (Math|Transform|MakeTransform (Math|Vector|MakeVector (Math|Conversions|ToFloat(Integer) (* _index 160)) (Math|Conversions|ToFloat(Integer) (* _index_2 160)) (Math|Conversions|ToFloat(Integer) (* _index_3 350))) (Math|Random|RandomRotator true)))))))
  (for _index_4 (range 0 9)
    (bind _returnvalue_2 (Class|CellularTerrain|GetX _cell (Utilities|Array|Get(acopy) (Variables|/Script/GameJam.CellularTerrain|GetFeatherLocations _cell) _index_4)))
    (bind _returnvalue_3 (Class|CellularTerrain|GetY _cell (Utilities|Array|Get(acopy) (Variables|/Script/GameJam.CellularTerrain|GetFeatherLocations _cell) _index_4)))
    (Game|SpawnActorfromClass "/Game/Blueprints/FeatherPickup.FeatherPickup_C" (Math|Conversions|ToTransform(Vector) (+ (Math|Vector|MakeVector (* 160 (Math|Conversions|ToFloat(Integer) _returnvalue_2)) (* 160 (Math|Conversions|ToFloat(Integer) _returnvalue_3)) 55.0) "-4000.000000,-4000.000000,0.000000")) "Undefined" 0 0)))

(fn ConstructionScript)